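; BP_Chest is a loot chest in the zombie game's inventory system that opens once, when its OnCollisionEnter event first fires.
; The AbrirCofre timeline rolls the Scene component open, then BPLooteableComponent spawns an item at SpawnPoint.
; The item is either the configured ItemToDrop or, with IsRandom set, a DT_Items row whose name is picked at random from ItemToDrop's data table.
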(event `/Game/Zombie/Blueprints/Interface/BPI_OnCollisionEvents.OnCollisionEnter`
  (bind _itemtodrop_datatable (break `DataTableRowHandle` (`self.ItemToDrop`)))
  (if (not (`self.Abierto`))
    (set `self.Abierto` true)
    (bind (_direction _angle) (`Timeline|AbrirCofre`)
      (:`Update`
        (`SceneComponent.K2_SetRelativeRotation` (`self.Scene`) (`KismetMathLibrary.MakeRotator` _angle) false false))
      (:`Finished`
        (if (`self.isRandom`)
          (bind _outrownames (`DataTableFunctionLibrary.GetDataTableRowNames` _itemtodrop_datatable))
          (`/Game/Zombie/Blueprints/Components/BP_Looteable_Component.SpawnObject` (`self.BP_Looteable_Component`) (`SceneComponent.K2_GetComponentToWorld` (`self.SpawnPoint`)) (make `DataTableRowHandle` "/Game/Zombie/Blueprints/InventorySystem/DT_Items.DT_Items" (`|GetArrayItem` _outrownames (`KismetMathLibrary.RandomIntegerInRange` 0 (- (`KismetArrayLibrary.Array_Length` _outrownames) 1)))))
          (else
            (`/Game/Zombie/Blueprints/Components/BP_Looteable_Component.SpawnObject` (`self.BP_Looteable_Component`) (`SceneComponent.K2_GetComponentToWorld` (`self.SpawnPoint`)) (`self.ItemToDrop`))))))))

(fn `UserConstructionScript`)