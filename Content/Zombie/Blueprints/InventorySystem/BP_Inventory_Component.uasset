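; BP_Inventory_Component is an inventory component that tracks items and their quantities in a map keyed by item.
; Adding an item increases its stored quantity or creates a new entry.
; Removing checks that the item exists in sufficient quantity, subtracts it, deletes emptied entries and returns success or failure.
; Failed removals print Spanish debug messages for a missing item or insufficient quantity.
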(fn `AddItemToInventory`
  (params (nameItemToAdd :type "Name (by ref)") (quantityToAdd :type "Integer (by ref)"))
  (bind (_value _returnvalue) (`BlueprintMapLibrary.Map_Find` (`self.Inventory`) nameItemToAdd))
  (if _returnvalue
    (`BlueprintMapLibrary.Map_Add` (`self.Inventory`) nameItemToAdd (+ quantityToAdd _value))
    (else
      (`BlueprintMapLibrary.Map_Add` (`self.Inventory`) nameItemToAdd quantityToAdd))))

(fn `RemoveItemFromInventory`
  (params (ItemToRemove :type "Name (by ref)") (QuantityToRemove :type "Integer (by ref)"))
  (returns (ItemRemoved :type Boolean))
  (bind (_value _returnvalue) (`BlueprintMapLibrary.Map_Find` (`self.Inventory`) ItemToRemove))
  (bind _returnvalue_2 (- _value QuantityToRemove))
  (if _returnvalue
    (if (<= QuantityToRemove _value)
      (if (<= _returnvalue_2 0)
        (`BlueprintMapLibrary.Map_Remove` (`self.Inventory`) ItemToRemove)
        (else
          (`BlueprintMapLibrary.Map_Add` (`self.Inventory`) ItemToRemove _returnvalue_2)))
      (return true)
      (else
        (`KismetSystemLibrary.PrintString` "no tengo suficiente")))
    (else
      (`KismetSystemLibrary.PrintString` "no tengo el item")))
  (return false))