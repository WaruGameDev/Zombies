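; BP_Item is a pickup actor that adds an item to the player's inventory and then destroys itself.
; Its construction script reads the ItemInfo data table row to set the static mesh and name text.
; OnCollisionEnter casts player pawn 0 to BP_ThirdPersonCharacter, rather than checking the colliding actor, and passes the row name and Quantity to BPInventoryComponent.
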(event `/Game/Zombie/Blueprints/Interface/BPI_OnCollisionEvents.OnCollisionEnter`
  (bind (_iteminfo_datatable _iteminfo_rowname) (break `DataTableRowHandle` (`self.ItemInfo`)))
  (bind _asbp_third_person_character (cast `/Game/ThirdPerson/Blueprints/BP_ThirdPersonCharacter` (`GameplayStatics.GetPlayerPawn` 0)))
  (`/Game/Zombie/Blueprints/InventorySystem/BP_Inventory_Component.AddItemToInventory` (`/Game/ThirdPerson/Blueprints/BP_ThirdPersonCharacter.BP_Inventory_Component` _asbp_third_person_character) _iteminfo_rowname (`self.Quantity`))
  (`self.K2_DestroyActor`))

(fn `SetItem`
  (bind (_iteminfo_datatable _iteminfo_rowname) (break `DataTableRowHandle` (`self.ItemInfo`)))
  (bind _returnvalue (`|GetDataTableRow` _iteminfo_datatable _iteminfo_rowname)
    (:`then`
      (bind (_nameitem _descriptionitem _buycost _sellcost _modelitem) (break `/Game/Zombie/Blueprints/InventorySystem/S_Item` _returnvalue))
      (`TextRenderComponent.K2_SetText` (`self.TextRender`) (`KismetTextLibrary.Conv_NameToText` _nameitem))
      (`StaticMeshComponent.SetStaticMesh` (`self.StaticMesh`) _modelitem))))

(fn `UserConstructionScript`
  (`self.SetItem`))