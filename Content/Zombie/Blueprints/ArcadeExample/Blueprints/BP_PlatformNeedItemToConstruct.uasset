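; Platform that constructs a building when the player pays it with items from their inventory.
; On collision, it removes the configured item and quantity from the third-person character's inventory component.
; If that succeeds, it spawns the chosen building class at a referenced position actor's transform, then destroys itself and that marker.
; The construction script labels a text render with the required item row name and quantity.
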(event `/Game/Zombie/Blueprints/Interface/BPI_OnCollisionEvents.OnCollisionEnter`
  (bind (_itemneeded_datatable _itemneeded_rowname) (break `DataTableRowHandle` (`self.ItemNeeded`)))
  (bind _asbp_third_person_character (cast `/Game/ThirdPerson/Blueprints/BP_ThirdPersonCharacter` (`GameplayStatics.GetPlayerPawn` 0)))
  (bind _itemremoved (`/Game/Zombie/Blueprints/InventorySystem/BP_Inventory_Component.RemoveItemFromInventory` (`/Game/ThirdPerson/Blueprints/BP_ThirdPersonCharacter.BP_Inventory_Component` _asbp_third_person_character) _itemneeded_rowname (`self.Quantity`)))
  (if _itemremoved
    (`|SpawnActorFromClass` (`self.BuildingToBuild`) (`self.GetTransform` (`self.PosToBuild`)) "Undefined" "MultiplyWithRoot" null null)
    (`self.K2_DestroyActor`)
    (`self.K2_DestroyActor` (`self.PosToBuild`))))

(fn `UserConstructionScript`
  (bind (_itemneeded_datatable _itemneeded_rowname) (break `DataTableRowHandle` (`self.ItemNeeded`)))
  (`TextRenderComponent.K2_SetText` (`self.TextRender`) (`KismetTextLibrary.Conv_StringToText` (`KismetStringLibrary.Concat_StrStr` (`KismetStringLibrary.Conv_NameToString` _itemneeded_rowname) " " "x" (`KismetStringLibrary.Conv_IntToString` (`self.Quantity`))))))